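; Level exit trigger that moves the player to the next map in a fixed sequence and saves progress when a BP_PlayerBase overlaps it.
; The overlap creates a fresh BP_SaveGame, then SetFBPlayer swaps the player's movement flipbooks by current map name and copies them into the save.
; OpenNewLevel opens the following map and records its name, after which the save is written to slot "SaveGame".
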(event OnComponentBeginOverlap(Trigger)
  (params (OverlappedComponent :type Primitive%20Component%20Object%20Reference) (OtherActor :type Actor%20Object%20Reference) (OtherComp :type Primitive%20Component%20Object%20Reference) (OtherBodyIndex :type Integer) (bFromSweep :type Boolean) (SweepResult :type Hit%20Result%20Structure%20%28by%20ref%29))
  (bind _asbp_player_base (Utilities|Casting|CastToBP_PlayerBase OtherActor))
  (Variables|Default|SetPlayerBaseRefOut _asbp_player_base)
  (bind _returnvalue (SaveGame|CreateSaveGameObject "/Game/Blueprints/BP_SaveGame.BP_SaveGame_C"))
  (Variables|Default|SetSaveGameInstanceOut _returnvalue)
  (bind _returnvalue_2 (Game|GetCurrentLevelName true))
  (Variables|Default|SetNameCurrentMap _returnvalue_2)
  (CallFunction|SetFBPlayer)
  (CallFunction|OpenNewLevel)
  (SaveGame|SaveGametoSlot (Variables|Default|GetSaveGameInstanceOut) "SaveGame")
  (Development|PrintString "Игра Сохранена"))

(event EventBeginPlay)

(event Collision|EventActorBeginOverlap
  (params (OtherActor :type Actor%20Object%20Reference)))

(event EventTick
  (params (DeltaSeconds :type Float%20%28single-precision%29)))

(fn ConstructionScript)

(fn OpenNewLevel
  (bind _savegameinstanceout (Variables|Default|GetSaveGameInstanceOut))
  (switch string (Variables|Default|GetNameCurrentMap)
    (:1Map
      (Game|OpenLevel(byName) "2Map")
      (Variables|/Game/Blueprints/BP_SaveGame.BP_SaveGame_C|SetMapName _savegameinstanceout "2Map"))
    (:2Map
      (Game|OpenLevel(byName) "3Map")
      (Variables|/Game/Blueprints/BP_SaveGame.BP_SaveGame_C|SetMapName _savegameinstanceout "3Map"))
    (:3Map
      (Game|OpenLevel(byName) "4Map")
      (Variables|/Game/Blueprints/BP_SaveGame.BP_SaveGame_C|SetMapName _savegameinstanceout "4Map"))
    (:4Map
      (Game|OpenLevel(byName) "5Map")
      (Variables|/Game/Blueprints/BP_SaveGame.BP_SaveGame_C|SetMapName _savegameinstanceout "5Map"))))

(fn SetFBPlayer
  (bind _playerbaserefout (Variables|Default|GetPlayerBaseRefOut))
  (bind _savegameinstanceout (Variables|Default|GetSaveGameInstanceOut))
  (bind _playerbaserefout_2 (Variables|Default|GetPlayerBaseRefOut))
  (bind _playerbaserefout_3 (Variables|Default|GetPlayerBaseRefOut))
  (bind _playerbaserefout_4 (Variables|Default|GetPlayerBaseRefOut))
  (bind _playerbaserefout_5 (Variables|Default|GetPlayerBaseRefOut))
  (switch string (Variables|Default|GetNameCurrentMap)
    (:1Map
      (Utilities|FlowControl|Sequence
        (:then_0
          (Variables|/Game/Blueprints/BP_PlayerBase.BP_PlayerBase_C|SetFB_Fall _playerbaserefout_2 "/Game/Assets/Flipbooks/Players/FB_PlayerLFall.FB_PlayerLFall"))
        (:then_1
          (Variables|/Game/Blueprints/BP_PlayerBase.BP_PlayerBase_C|SetFB_Idle _playerbaserefout_2 "/Game/Assets/Flipbooks/Players/FB_PlayerLIdle.FB_PlayerLIdle"))
        (:then_2
          (Variables|/Game/Blueprints/BP_PlayerBase.BP_PlayerBase_C|SetFB_Jump _playerbaserefout_2 "/Game/Assets/Flipbooks/Players/FB_PlayerLJump.FB_PlayerLJump"))
        (:then_3
          (Variables|/Game/Blueprints/BP_PlayerBase.BP_PlayerBase_C|SetFB_Run _playerbaserefout_2 "/Game/Assets/Flipbooks/Players/FB_PlayerLRun.FB_PlayerLRun"))))
    (:2Map
      (Utilities|FlowControl|Sequence
        (:then_0
          (Variables|/Game/Blueprints/BP_PlayerBase.BP_PlayerBase_C|SetFB_Fall _playerbaserefout_4 "/Game/Assets/Flipbooks/Players/FB_PlayerSFall.FB_PlayerSFall"))
        (:then_1
          (Variables|/Game/Blueprints/BP_PlayerBase.BP_PlayerBase_C|SetFB_Idle _playerbaserefout_4 "/Game/Assets/Flipbooks/Players/FB_PlayerSIdle.FB_PlayerSIdle"))
        (:then_2
          (Variables|/Game/Blueprints/BP_PlayerBase.BP_PlayerBase_C|SetFB_Jump _playerbaserefout_4 "/Game/Assets/Flipbooks/Players/FB_PlayerSJump.FB_PlayerSJump"))
        (:then_3
          (Variables|/Game/Blueprints/BP_PlayerBase.BP_PlayerBase_C|SetFB_Run _playerbaserefout_4 "/Game/Assets/Flipbooks/Players/FB_PlayerSRun.FB_PlayerSRun"))))
    (:3Map
      (Utilities|FlowControl|Sequence
        (:then_0
          (Variables|/Game/Blueprints/BP_PlayerBase.BP_PlayerBase_C|SetFB_Fall _playerbaserefout_5 "/Game/Assets/Flipbooks/Players/FB_PlayerAFall.FB_PlayerAFall"))
        (:then_1
          (Variables|/Game/Blueprints/BP_PlayerBase.BP_PlayerBase_C|SetFB_Idle _playerbaserefout_5 "/Game/Assets/Flipbooks/Players/FB_PlayerSIdle.FB_PlayerSIdle"))
        (:then_2
          (Variables|/Game/Blueprints/BP_PlayerBase.BP_PlayerBase_C|SetFB_Jump _playerbaserefout_5 "/Game/Assets/Flipbooks/Players/FB_PlayerSJump.FB_PlayerSJump"))
        (:then_3
          (Variables|/Game/Blueprints/BP_PlayerBase.BP_PlayerBase_C|SetFB_Run _playerbaserefout_5 "/Game/Assets/Flipbooks/Players/FB_PlayerSRun.FB_PlayerSRun"))))
    (:4Map
      (Utilities|FlowControl|Sequence
        (:then_0
          (Variables|/Game/Blueprints/BP_PlayerBase.BP_PlayerBase_C|SetFB_Fall _playerbaserefout_3 "/Game/Assets/Flipbooks/Players/FB_PlayerDFall.FB_PlayerDFall"))
        (:then_1
          (Variables|/Game/Blueprints/BP_PlayerBase.BP_PlayerBase_C|SetFB_Idle _playerbaserefout_3 "/Game/Assets/Flipbooks/Players/FB_PlayerDIdle.FB_PlayerDIdle"))
        (:then_2
          (Variables|/Game/Blueprints/BP_PlayerBase.BP_PlayerBase_C|SetFB_Jump _playerbaserefout_3 "/Game/Assets/Flipbooks/Players/FB_PlayerDJump.FB_PlayerDJump"))
        (:then_3
          (Variables|/Game/Blueprints/BP_PlayerBase.BP_PlayerBase_C|SetFB_Run _playerbaserefout_3 "/Game/Assets/Flipbooks/Players/FB_PlayerDRun.FB_PlayerDRun")))))
  (Utilities|FlowControl|Sequence
    (:then_0
      (Variables|/Game/Blueprints/BP_SaveGame.BP_SaveGame_C|SetFBPlayerFall _savegameinstanceout (Variables|/Game/Blueprints/BP_PlayerBase.BP_PlayerBase_C|GetFB_Fall _playerbaserefout)))
    (:then_1
      (Variables|/Game/Blueprints/BP_SaveGame.BP_SaveGame_C|SetFBPlayerIdle _savegameinstanceout (Variables|/Game/Blueprints/BP_PlayerBase.BP_PlayerBase_C|GetFB_Idle _playerbaserefout)))
    (:then_2
      (Variables|/Game/Blueprints/BP_SaveGame.BP_SaveGame_C|SetFBPlayerJump _savegameinstanceout (Variables|/Game/Blueprints/BP_PlayerBase.BP_PlayerBase_C|GetFB_Jump _playerbaserefout)))
    (:then_3
      (Variables|/Game/Blueprints/BP_SaveGame.BP_SaveGame_C|SetFBPlayerRun _savegameinstanceout (Variables|/Game/Blueprints/BP_PlayerBase.BP_PlayerBase_C|GetFB_Run _playerbaserefout)))))