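; Interactive dumpling pickup that alters the player's movement and camera when interacted with, then destroys itself.
; Interact writes directly to the passed player reference, overriding walk and run speed, jump hold time and knockback-related values, and repositioning the camera.
; It plays the Violent sound at the world origin rather than at the dumpling's location.
; The event graph holds no active logic, and nothing here reverts the changes.
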(event EventBeginPlay
  (|CallParentFunction) ; This node is disabled and will not be called.\nDrag off pins to build functionality.
)

(event Collision|EventActorBeginOverlap
  (params (OtherActor :type Actor%20Object%20Reference)))

(event EventTick
  (params (DeltaSeconds :type Float%20%28single-precision%29)))

(fn ConstructionScript
  (|CallParentFunction))

(fn Interact
  (params (PlayerRef :type BP%20Player%20Base%20Object%20Reference))
  (Variables|/Script/Engine.CharacterMovementComponent|SetMaxWalkSpeed (Variables|/Script/Engine.Character|GetCharacterMovement PlayerRef) (Variables|Default|GetWalkSpeed))
  (Variables|/Game/Blueprints/BP_PlayerBase.BP_PlayerBase_C|SetFB_Run PlayerRef "/Game/Assets/Flipbooks/Players/FB_PlayerARunSpeed.FB_PlayerARunSpeed")
  (Variables|/Game/Blueprints/BP_PlayerBase.BP_PlayerBase_C|SetHitCoordinateZ PlayerRef 1.0)
  (Variables|/Game/Blueprints/BP_PlayerBase.BP_PlayerBase_C|SetKnockBackForce PlayerRef 0.0)
  (Variables|/Script/Engine.Character|SetJumpMaxHoldTime PlayerRef 1.0)
  (Transformation|SetRelativeLocation (Variables|/Game/Blueprints/BP_PlayerBase.BP_PlayerBase_C|GetCamera PlayerRef) "-300.000000, 0, 0" false false)
  (Audio|PlaySoundatLocation "/Game/Sound/violent.violent" "0, 0, 0" "0, 0, 0" 1.0 1.0 0.0 0 0 0)
  (Actor|DestroyActor))