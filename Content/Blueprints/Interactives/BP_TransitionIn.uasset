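; BP_TransitionIn is a trigger actor that restores the player's saved flipbook set on overlap, apparently when entering a map.
; When a BP_PlayerBase overlaps its Trigger, it loads the BP_SaveGame from the "SaveGame" slot.
; It then copies the saved fall, idle, jump and run flipbook references onto the player.
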(event OnComponentBeginOverlap(Trigger)
  (params (OverlappedComponent :type Primitive%20Component%20Object%20Reference) (OtherActor :type Actor%20Object%20Reference) (OtherComp :type Primitive%20Component%20Object%20Reference) (OtherBodyIndex :type Integer) (bFromSweep :type Boolean) (SweepResult :type Hit%20Result%20Structure%20%28by%20ref%29))
  (bind _asbp_player_base (Utilities|Casting|CastToBP_PlayerBase OtherActor))
  (Variables|Default|SetPlayerBaseRefIn _asbp_player_base)
  (bind _returnvalue (SaveGame|LoadGamefromSlot "SaveGame"))
  (bind _asbp_save_game (Utilities|Casting|CastToBP_SaveGame _returnvalue))
  (Variables|Default|SetSaveGameInstanceIn _asbp_save_game)
  (Utilities|FlowControl|Sequence
    (:then_0
      (Variables|/Game/Blueprints/BP_PlayerBase.BP_PlayerBase_C|SetFB_Fall (Variables|Default|GetPlayerBaseRefIn) (Variables|/Game/Blueprints/BP_SaveGame.BP_SaveGame_C|GetFBPlayerFall (Variables|Default|GetSaveGameInstanceIn))))
    (:then_1
      (Variables|/Game/Blueprints/BP_PlayerBase.BP_PlayerBase_C|SetFB_Idle (Variables|Default|GetPlayerBaseRefIn) (Variables|/Game/Blueprints/BP_SaveGame.BP_SaveGame_C|GetFBPlayerIdle (Variables|Default|GetSaveGameInstanceIn))))
    (:then_2
      (Variables|/Game/Blueprints/BP_PlayerBase.BP_PlayerBase_C|SetFB_Jump (Variables|Default|GetPlayerBaseRefIn) (Variables|/Game/Blueprints/BP_SaveGame.BP_SaveGame_C|GetFBPlayerJump (Variables|Default|GetSaveGameInstanceIn))))
    (:then_3
      (Variables|/Game/Blueprints/BP_PlayerBase.BP_PlayerBase_C|SetFB_Run (Variables|Default|GetPlayerBaseRefIn) (Variables|/Game/Blueprints/BP_SaveGame.BP_SaveGame_C|GetFBPlayerRun (Variables|Default|GetSaveGameInstanceIn))))))

(event EventBeginPlay)

(event Collision|EventActorBeginOverlap
  (params (OtherActor :type Actor%20Object%20Reference)))

(event EventTick
  (params (DeltaSeconds :type Float%20%28single-precision%29)))

(fn ConstructionScript)