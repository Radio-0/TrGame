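; Interactive glass actor that, when interacted with, changes the player's size and is consumed.
; Its Interact function takes the player reference, sets fixed capsule dimensions and sprite scale, and overwrites the player's HitCoordinateZ value.
; The actor then destroys itself, making the interaction single-use; its event graph and construction script add no logic of their own.
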(event EventBeginPlay
  (|CallParentFunction) ; This node is disabled and will not be called.\nDrag off pins to build functionality.
)

(event Collision|EventActorBeginOverlap
  (params (OtherActor :type Actor%20Object%20Reference)))

(event EventTick
  (params (DeltaSeconds :type Float%20%28single-precision%29)))

(fn ConstructionScript
  (|CallParentFunction))

(fn Interact
  (params (PlayerRef :type BP%20Player%20Base%20Object%20Reference))
  (Components|Capsule|SetCapsuleSize (Variables|/Script/Engine.Character|GetCapsuleComponent PlayerRef) 5e+01 5e+01 true)
  (Transformation|SetRelativeScale3D (Variables|/Script/Paper2D.PaperCharacter|GetSprite PlayerRef) "2.000000,1.000000,2.000000")
  (Variables|/Game/Blueprints/BP_PlayerBase.BP_PlayerBase_C|SetHitCoordinateZ PlayerRef 1.0)
  (Actor|DestroyActor))