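; BP_InteractiveSoapMove is a short-lived moving soap actor that destroys any enemy it overlaps.
; On BeginPlay it sets a two-second self-destruct timer and reverses its X direction if the first found player has negative X velocity.
; Each tick it applies a yaw variable to its Paper flipbook and moves along world X with a swept offset scaled by speed, direction and delta time.
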(event Custom|EventDestroySoup
  (Actor|DestroyActor))

(event EventBeginPlay
  (Utilities|Time|SetTimerbyEvent (delegate Custom|EventDestroySoup) 2.0)
  (bind _outactors (Actor|GetAllActorsOfClass "/Game/Blueprints/BP_PlayerBase.BP_PlayerBase_C"))
  (bind _asbp_player_base (Utilities|Casting|CastToBP_PlayerBase (Utilities|Array|Get(acopy) _outactors)))
  (Math|Float|CompareFloat (.x (Transformation|GetVelocity _asbp_player_base)) 0.0
    (:<
      (Variables|Default|SetDirectionXMoveSoup -5e+01))))

(event Collision|EventActorBeginOverlap
  (params (OtherActor :type Actor%20Object%20Reference))
  (bind _asbp_enemy_base (Utilities|Casting|CastToBP_EnemyBase OtherActor))
  (Actor|DestroyActor _asbp_enemy_base))

(event EventTick
  (params (DeltaSeconds :type Float%20%28single-precision%29))
  (Transformation|SetRelativeRotation (Variables|Default|GetPaperFlipbook) (Math|Rotator|MakeRotator 0.0 0.0 (Variables|Default|GetZRotationSoup)) false false)
  (Transformation|AddActorWorldOffset (Math|Vector|MakeVector (* (* (Variables|Default|GetSpeedSoup) (Variables|Default|GetDirectionXMoveSoup)) DeltaSeconds) 0.0 0.0) true))

(fn ConstructionScript)