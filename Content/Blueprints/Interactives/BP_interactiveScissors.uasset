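; BP_interactiveScissors is an interactive scissors pickup that switches the player to scissors-themed animations.
; Interact overwrites the player's fall, idle, jump and run flipbook variables with scissors variants, sets HitCoordinateZ and destroys the actor.
; All four Sequence branches converge on the same HitCoordinateZ and DestroyActor nodes, so that tail is wired to run after each swap.
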(event EventBeginPlay
  (|CallParentFunction) ; This node is disabled and will not be called.\nDrag off pins to build functionality.
)

(event Collision|EventActorBeginOverlap
  (params (OtherActor :type Actor%20Object%20Reference)))

(event EventTick
  (params (DeltaSeconds :type Float%20%28single-precision%29)))

(fn ConstructionScript
  (|CallParentFunction))

(fn Interact
  (params (PlayerRef :type BP%20Player%20Base%20Object%20Reference))
  (Utilities|FlowControl|Sequence
    (:then_0
      (Variables|/Game/Blueprints/BP_PlayerBase.BP_PlayerBase_C|SetFB_Fall PlayerRef "/Game/Assets/Flipbooks/Players/FB_PlayerS_ScissorsFall.FB_PlayerS_ScissorsFall"))
    (:then_1
      (Variables|/Game/Blueprints/BP_PlayerBase.BP_PlayerBase_C|SetFB_Idle PlayerRef "/Game/Assets/Flipbooks/Players/FB_PlayerS_ScissorsIdle.FB_PlayerS_ScissorsIdle"))
    (:then_2
      (Variables|/Game/Blueprints/BP_PlayerBase.BP_PlayerBase_C|SetFB_Jump PlayerRef "/Game/Assets/Flipbooks/Players/FB_PlayerS_ScissorsJump.FB_PlayerS_ScissorsJump"))
    (:then_3
      (Variables|/Game/Blueprints/BP_PlayerBase.BP_PlayerBase_C|SetFB_Run PlayerRef "/Game/Assets/Flipbooks/Players/FB_PlayerS_ScissorsRun.FB_PlayerS_ScissorsRun")))
  (Variables|/Game/Blueprints/BP_PlayerBase.BP_PlayerBase_C|SetHitCoordinateZ PlayerRef 1.0)
  (Actor|DestroyActor))